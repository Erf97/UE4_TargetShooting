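; Game state Blueprint that tracks base health and score for a match with a base to defend.
; On BeginPlay it resets health and seeds the starting score from that health.
; Damage decrements health, then either broadcasts it through a dispatcher or, once depleted, tells BP_GameMode the game has ended.
; Score changes are likewise broadcast, with simple math expression nodes handling the arithmetic.
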(event EventBeginPlay
  (CallFunction|ResetGameState))

(fn ConstructionScript)

(fn BaseGotDamage
  (bind _output_get (Variables|Default|SetBaseHealth (|(a-1) (Variables|Default|GetBaseHealth))))
  (if (|(a>0) _output_get)
    (Default|CallSendBaseHealth _output_get)
    (else
      (bind _asbp_game_mode (Utilities|Casting|CastToBP_GameMode (Game|GetGameMode)))
      (Default|OnGameEnd _asbp_game_mode _output_get))))

(fn ObtainScore
  (params (ScoreDelta :type Integer))
  (bind _output_get (Variables|Default|SetScore (|(a+b) ScoreDelta (Variables|Default|GetScore))))
  (Default|CallSendScore _output_get))

(fn ResetGameState
  (bind _output_get (Variables|Default|SetBaseHealth 10))
  (Variables|Default|SetScore (|(a*b) _output_get 10)))