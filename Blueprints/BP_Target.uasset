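; BP_Target is a shootable target that scores points when hit and damages the base if it gets through.
; While ShouldMove is set, Tick moves it along negative Y until it passes a boundary, then destroys it, deducts score and reports base damage to BP_GameState.
; OnTargetHit briefly activates RotatingMovement, destroys the actor, then awards score through a GetThisGameState cast helper.
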(event EventOnTargetHit
  (bind _rotatingmovement (Variables|Default|GetRotatingMovement))
  (Components|Activation|Activate _rotatingmovement false)
  (Utilities|FlowControl|Delay 0.3)
  (Components|Activation|Deactivate _rotatingmovement)
  (Actor|DestroyActor)
  (bind _asbp_game_state (Utilities|GetThisGameState)
    (:then
      (Default|ObtainScore _asbp_game_state 5))))

(event EventTick
  (params (DeltaSeconds :type Float%20%28single-precision%29))
  (if (Variables|Default|GetbShouldMove)
    (Transformation|AddActorWorldOffset (Math|Vector|MakeVector 0.0 (|(a*b) DeltaSeconds -3e+02) 0.0))
    (if (|(a<=b) (.Y (Math|Vector|BreakVector (.Location (Math|Transform|BreakTransform (Transformation|GetActorTransform))))) -8e+02)
      (Actor|DestroyActor)
      (bind _asbp_game_state (Utilities|Casting|CastToBP_GameState (Game|GetGameState)))
      (Default|ObtainScore _asbp_game_state -10)
      (Default|BaseGotDamage _asbp_game_state))))

(fn ConstructionScript)