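; Game mode that runs a timed round with base health and targets, switching between a start-tip screen and active play.
; The start-timing event begins a one-second Delay loop that broadcasts the countdown and calls game end at zero with BP_GameState's BaseHealth.
; Game end restores the start screen, destroys all BP_Target actors, shows victory or failure by remaining health with the score, then resets the game state.
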(event Custom|OnGameStart
  (CallFunction|SetGame)
  (Utilities|FlowControl|Delay 1.0 :!label _label)
  (bind _returnvalue (CallFunction|TimeCount))
  (if _returnvalue
    (bind _asbp_game_state (Utilities|GetThisGameState)
      (:then
        (Default|CallGameEnd (Variables|/Game/Blueprints/BP_GameState.BP_GameState_C|GetBaseHealth _asbp_game_state))))
    (else
      (goto _label))))

(event Custom|OnGameEnd
  (params (BaseHealth :type Integer))
  (CallFunction|ResetGame)
  (bind _outactors (Actor|GetAllActorsOfClass "/Game/Blueprints/BP_Target.BP_Target_C"))
  (Actor|DestroyActor _outactors)
  (if (|(a>b) BaseHealth)
    (CallFunction|OnGameVictory)
    (else
      (CallFunction|OnGameFailed)))
  (bind _asbp_game_state (Utilities|GetThisGameState)
    (:then
      (Default|ResetGameState _asbp_game_state))))

(event Custom|OnGameFailed
  (CallFunction|ShowGameEndWindow "Failed!"))

(event Custom|OnGameVictory
  (CallFunction|ShowGameEndWindow "Victory!"))

(event EventBeginPlay
  (EventDispatchers|BindEventtoStartTiming (delegate Custom|OnGameStart))
  (EventDispatchers|BindEventtoGameEnd (delegate Custom|OnGameEnd))
  (CallFunction|ResetGame))

(fn ConstructionScript)

(fn ResetGame
  (Variables|Default|SetbShouldStartGame true)
  (Variables|Default|SetbIsGameInProcess false)
  (Variables|Default|SetGameTimeSec 120)
  (bind _returnvalue (UserInterface|CreateWidget "/Game/Blueprints/UI/BP_TipsStartGame.BP_TipsStartGame_C"))
  (UserInterface|Viewport|AddtoViewport _returnvalue 0)
  (UserInterface|Animation|PlayAnimation _returnvalue (Variables|/Game/Blueprints/UI/BP_TipsStartGame.BP_TipsStartGame_C|GetBreathe _returnvalue) 0.0 0 "Forward" 1.0 false)
  (Variables|Default|SetGameStartTip _returnvalue))

(fn TimeCount
  (bind _output_get (Variables|Default|SetGameTimeSec (|(a-1) (Variables|Default|GetGameTimeSec))))
  (Default|CallSendTime _output_get)
  (return (|(a==0) _output_get)))

(fn SetGame
  (Variables|Default|SetbShouldStartGame false)
  (Variables|Default|SetbIsGameInProcess true)
  (Widget|RemovefromParent (Variables|Default|GetGameStartTip)))

(fn ShowGameEndWindow
  (params (InText :type Text))
  (bind _returnvalue (UserInterface|CreateWidget "/Game/Blueprints/UI/BP_GameEndWindow.BP_GameEndWindow_C"))
  (Rendering|Components|TextRender|SetText (Variables|/Game/Blueprints/UI/BP_GameEndWindow.BP_GameEndWindow_C|GetGameEndText _returnvalue) InText)
  (bind _asbp_game_state (Utilities|GetThisGameState)
    (:then
      (Default|SetScoreText _returnvalue (Variables|/Game/Blueprints/BP_GameState.BP_GameState_C|GetScore _asbp_game_state))
      (UserInterface|Viewport|AddtoViewport _returnvalue 0))))