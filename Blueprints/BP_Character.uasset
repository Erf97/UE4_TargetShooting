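; BP_Character is a character Blueprint that shows a weapon tip on screen while the player aims at a gun.
; BeginPlay creates the BP_TipsWeapon widget for player controller 0 and adds it to the viewport collapsed.
; Each Tick, it compares the class of the GetAimingActor result to Gun by exact match, then calls one of two events that show or collapse the tip.
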(event `self.ReceiveBeginPlay`
  (bind _returnvalue (`|CreateWidget` "/Game/Blueprints/UI/BP_TipsWeapon.BP_TipsWeapon_C" (`GameplayStatics.GetPlayerController` 0)))
  (bind _output_get (set `self.WeaponTip` _returnvalue))
  (`Widget.SetVisibility` _output_get "Collapsed")
  (`UserWidget.AddToViewport` _output_get 0))

(event `self.ReceiveTick`
  (params (DeltaSeconds :type "Float (single-precision)"))
  (bind _returnvalue (`self.GetAimingActor`))
  (if (== (`GameplayStatics.GetObjectClass` _returnvalue) "/Script/ShotingTarget.Gun")
    (`self.OnAimmingWeapon`)
    (else
      (`self.OnAimmingOtherActor`))))

(event `OnAimmingWeapon`
  (`Widget.SetVisibility` (`self.WeaponTip`) "Visible"))

(event `OnAimmingOtherActor`
  (`Widget.SetVisibility` (`self.WeaponTip`) "Collapsed"))

(fn `UserConstructionScript`)